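; BP_AwardGameMode is a game mode that manages level streaming and respawning for the BP_Award player pawn.
; On BeginPlay it streams in Stage1 and moves the pawn to the player start.
; When the pawn is destroyed, it spawns and possesses a new BP_Award there, then rebinds the destroy event.
; A NextStage event, not called here, swaps Stage1 for Stage2 and repositions the pawn.
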(event `self.ReceiveBeginPlay`
  (`self.RespawnEvent`)
  (`self.LoadStage`))

(event `LoadStage`
  ;[1 1 1] LoadStage
  (`GameplayStatics.LoadStreamLevel` "Stage1" true true)
  (`self.Set Award Transform`))

(event `RespawnEvent`
  ;[1 1 1] Respawn
  (add `self.OnDestroyed` (`GameplayStatics.GetPlayerPawn` 0) (delegate `RespawnAward`)))

(event `RespawnAward` :!signature `self.OnDestroyed`
  (params (DestroyedActor :type "Actor Object Reference"))
  ;[1 1 1] Respawn
  (bind _returnvalue (`|SpawnActorFromClass` "/Game/BP/BP_Award.BP_Award_C" (`self.GetTransform` (`self.K2_FindPlayerStart` null)) "Undefined" "OverrideRootScale" null null))
  (`Controller.Possess` (`GameplayStatics.GetPlayerController` 0) _returnvalue)
  (`self.RespawnEvent`))

(event `NextStage`
  ;[1 1 1] NextStage
  (`GameplayStatics.UnloadStreamLevel` "Stage1")
  (`GameplayStatics.LoadStreamLevel` "Stage2" true true)
  (`self.Set Award Transform`))

(fn `Set Award Transform`
  (`self.K2_SetActorTransform` (`GameplayStatics.GetPlayerPawn` 0) (`self.GetTransform` (`self.K2_FindPlayerStart` null)) false false))

(fn `UserConstructionScript`)